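; Level exit door for the side scroller that completes the level when the overlapping player has the key, otherwise plays a locked sound and briefly shows a need-key message.
; On success it pauses, adds a LevelTimer-based bonus to the GameInstance score, and shows the completion widget.
; Outside high score mode it also unlocks the next level, derives its name from the current name's numeric suffix, and async-saves progress before showing Level Complete or Game Complete.
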(event Collision|EventActorBeginOverlap
  (params (OtherActor :type Actor%20Object%20Reference))
  ;[1 1 1] If Player Has Key Show Level Complete Screen And Calculate Score
  (bind _assimple_side_scroller_character (Utilities|Casting|CastToSimpleSideScrollerCharacter OtherActor))
  (if (Variables|/Game/Blueprints/Player/SimpleSideScrollerCharacter.SimpleSideScrollerCharacter_C|GetHasLevelKey _assimple_side_scroller_character)
    (Game|SetGamePaused true)
    (Audio|PlaySound2D "/Game/Audio/SoundEffects/UnlockedDoor.UnlockedDoor" 1.0 1.0 0.0 0 0)
    (Audio|PlaySound2D "/Game/Audio/SoundEffects/DoorOpen.DoorOpen" 1.0 1.0 0.0 0 0)
    (bind _assimple_side_scroller_game_instance (Utilities|Casting|CastToSimpleSideScrollerGameInstance (Game|GetGameInstance)))
    (if (Variables|/Game/Blueprints/Player/SimpleSideScrollerGameInstance.SimpleSideScrollerGameInstance_C|GetHighScoreMode _assimple_side_scroller_game_instance)
      (bind _assimple_side_scroller_game_mode (Utilities|Casting|CastToSimpleSideScrollerGameMode (Game|GetGameMode)))
      (bind _assimple_side_scroller_game_instance_2 (Utilities|Casting|CastToSimpleSideScrollerGameInstance (Game|GetGameInstance)))
      (Variables|/Game/Blueprints/Player/SimpleSideScrollerGameInstance.SimpleSideScrollerGameInstance_C|SetScore _assimple_side_scroller_game_instance_2 (+ (Variables|/Game/Blueprints/Player/SimpleSideScrollerGameInstance.SimpleSideScrollerGameInstance_C|GetScore _assimple_side_scroller_game_instance_2) (* (Variables|/Game/Blueprints/Player/SimpleSideScrollerGameMode.SimpleSideScrollerGameMode_C|GetLevelTimer _assimple_side_scroller_game_mode) 100)))
      (bind _returnvalue (UserInterface|CreateWidget "/Game/Blueprints/HUD/LevelComplete.LevelComplete_C"))
      (UserInterface|Viewport|AddtoViewport _returnvalue 0)
      (Variables|/Script/Engine.PlayerController|SetbShowMouseCursor (Game|GetPlayerController 0) true)
      (else
        (Utilities|Array|SetArrayElem (Variables|/Game/Blueprints/Player/SimpleSideScrollerGameInstance.SimpleSideScrollerGameInstance_C|GetLevelCompleted _assimple_side_scroller_game_instance) (Variables|/Game/Blueprints/Player/SimpleSideScrollerGameInstance.SimpleSideScrollerGameInstance_C|GetLevelIndex _assimple_side_scroller_game_instance) true)
        (Utilities|Array|SetArrayElem (Variables|/Game/Blueprints/Player/SimpleSideScrollerGameInstance.SimpleSideScrollerGameInstance_C|GetLevelUnlocked _assimple_side_scroller_game_instance) (+ (Variables|/Game/Blueprints/Player/SimpleSideScrollerGameInstance.SimpleSideScrollerGameInstance_C|GetLevelIndex _assimple_side_scroller_game_instance) 1) true)
        (Utilities|FlowControl|Sequence
          (:then_0
            (bind _returnvalue_2 (Game|GetCurrentLevelName true))
            (bind _output_get (Variables|/Game/Blueprints/Player/SimpleSideScrollerGameInstance.SimpleSideScrollerGameInstance_C|SetCurrentLevelName _assimple_side_scroller_game_instance (Utilities|String|Append (Utilities|String|LeftChop _returnvalue_2 1) (Utilities|String|ToString(Integer) (+ (Math|Conversions|ToInteger(Byte) (Utilities|String|RightChop _returnvalue_2 5)) 1)))))
            (bind _output_get_2 (Variables|/Game/Blueprints/Player/SimpleSideScrollerGameInstance.SimpleSideScrollerGameInstance_C|SetLevelCompleted _assimple_side_scroller_game_instance (Variables|/Game/Blueprints/Player/SimpleSideScrollerGameInstance.SimpleSideScrollerGameInstance_C|GetLevelCompleted _assimple_side_scroller_game_instance)))
            (bind _output_get_3 (Variables|/Game/Blueprints/Player/SimpleSideScrollerGameInstance.SimpleSideScrollerGameInstance_C|SetLevelUnlocked _assimple_side_scroller_game_instance (Variables|/Game/Blueprints/Player/SimpleSideScrollerGameInstance.SimpleSideScrollerGameInstance_C|GetLevelUnlocked _assimple_side_scroller_game_instance)))
            (if (>= (Variables|/Game/Blueprints/Player/SimpleSideScrollerGameInstance.SimpleSideScrollerGameInstance_C|GetLevelIndex _assimple_side_scroller_game_instance) (Variables|/Game/Blueprints/Player/SimpleSideScrollerGameInstance.SimpleSideScrollerGameInstance_C|GetPlayerMaxLevelIndex _assimple_side_scroller_game_instance))
              (bind _output_get_4 (Variables|/Game/Blueprints/Player/SimpleSideScrollerGameInstance.SimpleSideScrollerGameInstance_C|SetPlayerMaxLevelIndex _assimple_side_scroller_game_instance (+ (Variables|/Game/Blueprints/Player/SimpleSideScrollerGameInstance.SimpleSideScrollerGameInstance_C|GetPlayerMaxLevelIndex _assimple_side_scroller_game_instance) 1)))))
          (:then_1
            (bind _assimple_side_scroller_game_mode_2 (Utilities|Casting|CastToSimpleSideScrollerGameMode (Game|GetGameMode)))
            (bind _assimple_side_scroller_game_instance_3 (Utilities|Casting|CastToSimpleSideScrollerGameInstance (Game|GetGameInstance)))
            (bind _output_get_5 (Variables|/Game/Blueprints/Player/SimpleSideScrollerGameInstance.SimpleSideScrollerGameInstance_C|SetScore _assimple_side_scroller_game_instance_3 (+ (Variables|/Game/Blueprints/Player/SimpleSideScrollerGameInstance.SimpleSideScrollerGameInstance_C|GetScore _assimple_side_scroller_game_instance_3) (* (Variables|/Game/Blueprints/Player/SimpleSideScrollerGameMode.SimpleSideScrollerGameMode_C|GetLevelTimer _assimple_side_scroller_game_mode_2) 100))))
            (bind _output_get_6 (Variables|/Game/Blueprints/Player/SimpleSideScrollerGameInstance.SimpleSideScrollerGameInstance_C|SetPlayerColourSelected _assimple_side_scroller_game_instance_3 (Variables|/Game/Blueprints/Player/SimpleSideScrollerGameInstance.SimpleSideScrollerGameInstance_C|GetPlayerColourSelected _assimple_side_scroller_game_instance_3))))
          (:then_2
            (bind _returnvalue_3 (SaveGame|CreateSaveGameObject "/Game/Blueprints/Player/SimpleSideScrollerSaveGame.SimpleSideScrollerSaveGame_C"))
            (bind _output_get_7 (Variables|Default|SetSaveGameInstance _returnvalue_3))
            (Variables|/Game/Blueprints/Player/SimpleSideScrollerSaveGame.SimpleSideScrollerSaveGame_C|SetPlayerScore _output_get_7 _output_get_5)
            (Variables|/Game/Blueprints/Player/SimpleSideScrollerSaveGame.SimpleSideScrollerSaveGame_C|SetPlayerMaxLevelIndex _output_get_7 _output_get_4)
            (Variables|/Game/Blueprints/Player/SimpleSideScrollerSaveGame.SimpleSideScrollerSaveGame_C|SetCurrentLevelName _output_get_7 _output_get)
            (Variables|/Game/Blueprints/Player/SimpleSideScrollerSaveGame.SimpleSideScrollerSaveGame_C|SetPlayerColourSelected _output_get_7 _output_get_6)
            (bind _assimple_side_scroller_game_instance_4 (Utilities|Casting|CastToSimpleSideScrollerGameInstance (Game|GetGameInstance)))
            (Variables|/Game/Blueprints/Player/SimpleSideScrollerSaveGame.SimpleSideScrollerSaveGame_C|SetPlayerLives _output_get_7 (Variables|/Game/Blueprints/Player/SimpleSideScrollerGameInstance.SimpleSideScrollerGameInstance_C|GetLives _assimple_side_scroller_game_instance_4))
            (Variables|/Game/Blueprints/Player/SimpleSideScrollerSaveGame.SimpleSideScrollerSaveGame_C|SetPlayerCoins _output_get_7 (Variables|/Game/Blueprints/Player/SimpleSideScrollerGameInstance.SimpleSideScrollerGameInstance_C|GetCoins _assimple_side_scroller_game_instance_4))
            (Variables|/Game/Blueprints/Player/SimpleSideScrollerSaveGame.SimpleSideScrollerSaveGame_C|SetPlayerDiamonds _output_get_7 (Variables|/Game/Blueprints/Player/SimpleSideScrollerGameInstance.SimpleSideScrollerGameInstance_C|GetDiamonds _assimple_side_scroller_game_instance_4))
            (Variables|/Game/Blueprints/Player/SimpleSideScrollerSaveGame.SimpleSideScrollerSaveGame_C|SetLevelCompleted _output_get_7 _output_get_2)
            (Variables|/Game/Blueprints/Player/SimpleSideScrollerSaveGame.SimpleSideScrollerSaveGame_C|SetLevelUnlocked _output_get_7 _output_get_3)
            (Variables|/Game/Blueprints/Player/SimpleSideScrollerSaveGame.SimpleSideScrollerSaveGame_C|SetPlayerAbilityAvailable _output_get_7 (Variables|/Game/Blueprints/Player/SimpleSideScrollerGameInstance.SimpleSideScrollerGameInstance_C|GetPlayerAbilityAvailable _assimple_side_scroller_game_instance_4))
            (|AsyncSaveGametoSlot _output_get_7 (Variables|/Game/Blueprints/Player/SimpleSideScrollerSaveGame.SimpleSideScrollerSaveGame_C|GetSaveSlotName _output_get_7) (Variables|/Game/Blueprints/Player/SimpleSideScrollerSaveGame.SimpleSideScrollerSaveGame_C|GetUserIndex _output_get_7)
              (:Completed
                (bind _returnvalue_4 (Game|GetCurrentLevelName true))
                (if (Utilities|Enum|Equal(Enum) _returnvalue_4 (Variables|Default|GetLastLevelName))
                  (bind _returnvalue_5 (UserInterface|CreateWidget "/Game/Blueprints/HUD/GameComplete.GameComplete_C"))
                  (UserInterface|Viewport|AddtoViewport _returnvalue_5 0)
                  (Variables|/Script/Engine.PlayerController|SetbShowMouseCursor (Game|GetPlayerController 0) true)
                  (else
                    (bind _returnvalue_6 (UserInterface|CreateWidget "/Game/Blueprints/HUD/LevelComplete.LevelComplete_C"))
                    (UserInterface|Viewport|AddtoViewport _returnvalue_6 0)
                    (Variables|/Script/Engine.PlayerController|SetbShowMouseCursor (Game|GetPlayerController 0) true)))))))))
    (else
      (Audio|PlaySoundatLocation "/Game/Audio/SoundEffects/LockedDoor.LockedDoor" "0, 0, 0" "0, 0, 0" 1.0 1.0 0.0 0 0 0)
      (if (not (Variables|Default|GetMessageDisplaying))
        (bind _returnvalue_7 (UserInterface|CreateWidget "/Game/Blueprints/HUD/YouNeedTheKeyMessage.YouNeedTheKeyMessage_C"))
        (bind _output_get_8 (Variables|Default|SetYouNeedTheKeyMessage _returnvalue_7))
        (UserInterface|Viewport|AddtoViewport _output_get_8 0)
        (Variables|Default|SetMessageDisplaying true)
        (Utilities|FlowControl|Delay 3.0)
        (Widget|RemovefromParent _output_get_8)
        (Variables|Default|SetMessageDisplaying false)))))

(fn ConstructionScript)
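; Small 2D moving platform that shuttles a paper sprite between its origin and a configurable end location.
; A timeline, rate-scaled by travel time, lerps the sprite's relative location, with LiftForward and LiftBackwards alternating after a stop delay.
; A SimpleSideScrollerCharacter overlapping the collider mid-move flips the travel direction.
; The construction script tints the sprite and uses TestEndLocation to preview either endpoint.
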(event OnComponentBeginOverlap(Collider)
  (params (OverlappedComponent :type Primitive%20Component%20Object%20Reference) (OtherActor :type Actor%20Object%20Reference) (OtherComp :type Primitive%20Component%20Object%20Reference) (OtherBodyIndex :type Integer) (bFromSweep :type Boolean) (SweepResult :type Hit%20Result%20Structure%20%28by%20ref%29))
  (bind _lifttimeline (Variables|Default|GetLiftTimeLine))
  (Utilities|Casting|CastToSimpleSideScrollerCharacter OtherActor)
  (if (Audio|Components|Audio|IsPlaying _lifttimeline)
    (if (Class|TimelineComponent|IsReversing _lifttimeline)
      (bind (_direction _driver) (Timeline|LiftTimeLine Play)
        (:Update
          (Transformation|SetRelativeLocation (Variables|Default|GetPaperSprite) (Math|Vector|Lerp(Vector) "0, 0, 0" (Variables|LiftControls|GetEndLocation) _driver) false false))
        (:Finished
          (Utilities|FlowControl|Delay (Variables|LiftControls|GetStopDelay))
          (switch Utilities|FlowControl|Switch|SwitchonETimelineDirection _direction
            (:Forward
              (CallFunction|LiftBackwards))
            (:Backward
              (CallFunction|LiftForward)))))
      (else
        (Timeline|LiftTimeLine Reverse)))))

(event Custom|LiftForward
  (bind (_direction _driver) (Timeline|LiftTimeLine PlayFromStart)
    (:Update
      (Transformation|SetRelativeLocation (Variables|Default|GetPaperSprite) (Math|Vector|Lerp(Vector) "0, 0, 0" (Variables|LiftControls|GetEndLocation) _driver) false false))
    (:Finished
      (Utilities|FlowControl|Delay (Variables|LiftControls|GetStopDelay))
      (switch Utilities|FlowControl|Switch|SwitchonETimelineDirection _direction
        (:Forward
          (CallFunction|LiftBackwards))
        (:Backward
          (CallFunction|LiftForward))))))

(event Custom|LiftBackwards
  (bind (_direction _driver) (Timeline|LiftTimeLine ReverseFromEnd)
    (:Update
      (Transformation|SetRelativeLocation (Variables|Default|GetPaperSprite) (Math|Vector|Lerp(Vector) "0, 0, 0" (Variables|LiftControls|GetEndLocation) _driver) false false))
    (:Finished
      (Utilities|FlowControl|Delay (Variables|LiftControls|GetStopDelay))
      (switch Utilities|FlowControl|Switch|SwitchonETimelineDirection _direction
        (:Forward
          (CallFunction|LiftBackwards))
        (:Backward
          (CallFunction|LiftForward))))))

(event EventBeginPlay
  (Components|Timeline|SetPlayRate (Variables|Default|GetLiftTimeLine) (/ 1.0 (Variables|LiftControls|GetTravelTimeSeconds)))
  (Variables|LiftControls|SetTestEndLocation true))

(event Collision|EventActorBeginOverlap
  (params (OtherActor :type Actor%20Object%20Reference)))

(event EventTick
  (params (DeltaSeconds :type Float%20%28single-precision%29)))

(fn ConstructionScript
  (Transformation|SetRelativeLocation (Variables|Default|GetPaperSprite) (Math|Vector|SelectVector (Variables|LiftControls|GetEndLocation) "0, 0, 0" (Variables|LiftControls|GetTestEndLocation)) false false)
  (Sprite|SetSpriteColor (Variables|Default|GetPaperSprite) (Variables|LiftControls|GetLiftColour)))
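; One-shot floor switch for a side-scroller that spawns five timed collectible items when the player character overlaps it.
; On overlap it swaps to the pressed green button sprite, disables further overlap events, sets query-only collision and plays a press sound.
; A sequence then spawns five configurable Blueprint classes, each at its own offset from the switch.
; Each spawned actor gets a shared lifespan, so uncollected items destroy themselves.
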(event OnComponentBeginOverlap(PaperSprite)
  (params (OverlappedComponent :type Primitive%20Component%20Object%20Reference) (OtherActor :type Actor%20Object%20Reference) (OtherComp :type Primitive%20Component%20Object%20Reference) (OtherBodyIndex :type Integer) (bFromSweep :type Boolean) (SweepResult :type Hit%20Result%20Structure%20%28by%20ref%29))
  ;[1 1 1] Spawn 5 Coins Then Destroy Them After A Delay If Not Collected
  (Utilities|Casting|CastToSimpleSideScrollerCharacter OtherActor)
  (Rendering|Components|Sprite|SetSprite (Variables|Default|GetPaperSprite) "/Game/Sprites/Items/ButtonGreenPressedSprite.ButtonGreenPressedSprite")
  (Variables|/Script/Engine.PrimitiveComponent|SetbGenerateOverlapEvents OverlappedComponent false)
  (Collision|SetCollisionEnabled (Variables|Default|GetPaperSprite) "QueryOnly")
  (Audio|PlaySoundatLocation "/Game/Audio/SoundEffects/PressSwitch.PressSwitch" "0, 0, 0" "0, 0, 0" 1.0 1.0 0.0 0 0 0)
  (Utilities|FlowControl|Sequence
    (:then_0
      (bind _returnvalue (Game|SpawnActorfromClass (Variables|Default|GetBlueprintToSpawn1) (Math|Transform|MakeTransform (+ (Transformation|GetActorLocation) (Variables|Default|GetDiamondOffset1)) (Variables|/Script/Engine.SceneComponent|GetRelativeRotation (Variables|Default|GetPaperSprite))) "Undefined" 0 0))
      (Actor|SetLifeSpan _returnvalue (Variables|Default|GetLifeSpan)))
    (:then_1
      (bind _returnvalue_2 (Game|SpawnActorfromClass (Variables|Default|GetBlueprintToSpawn2) (Math|Transform|MakeTransform (+ (Transformation|GetActorLocation) (Variables|Default|GetDiamondOffset2)) (Variables|/Script/Engine.SceneComponent|GetRelativeRotation (Variables|Default|GetPaperSprite))) "Undefined" 0 0))
      (Actor|SetLifeSpan _returnvalue_2 (Variables|Default|GetLifeSpan)))
    (:then_2
      (bind _returnvalue_3 (Game|SpawnActorfromClass (Variables|Default|GetBlueprintToSpawn3) (Math|Transform|MakeTransform (+ (Transformation|GetActorLocation) (Variables|Default|GetDiamondOffset3)) (Variables|/Script/Engine.SceneComponent|GetRelativeRotation (Variables|Default|GetPaperSprite))) "Undefined" 0 0))
      (Actor|SetLifeSpan _returnvalue_3 (Variables|Default|GetLifeSpan)))
    (:then_3
      (bind _returnvalue_4 (Game|SpawnActorfromClass (Variables|Default|GetBlueprintToSpawn4) (Math|Transform|MakeTransform (+ (Transformation|GetActorLocation) (Variables|Default|GetDiamondOffset4)) (Variables|/Script/Engine.SceneComponent|GetRelativeRotation (Variables|Default|GetPaperSprite))) "Undefined" 0 0))
      (Actor|SetLifeSpan _returnvalue_4 (Variables|Default|GetLifeSpan)))
    (:then_4
      (bind _returnvalue_5 (Game|SpawnActorfromClass (Variables|Default|GetBlueprintToSpawn5) (Math|Transform|MakeTransform (+ (Transformation|GetActorLocation) (Variables|Default|GetDiamondOffset5)) (Variables|/Script/Engine.SceneComponent|GetRelativeRotation (Variables|Default|GetPaperSprite))) "Undefined" 0 0))
      (Actor|SetLifeSpan _returnvalue_5 (Variables|Default|GetLifeSpan)))))

(fn ConstructionScript)
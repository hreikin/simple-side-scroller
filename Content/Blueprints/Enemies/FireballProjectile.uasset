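; Fireball projectile for a side-scroller that kills enemies it overlaps and expires after five seconds.
; A sphere overlap runs a cast chain over four enemy types and the boss, repeating the same kill sequence for each.
; Each hit calls HealthSystem, spawns a DeadEnemy flipbook, destroys enemy and fireball, and adds type-specific score to the game instance.
; The boss also dies in one hit and drops PickupKeys.
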(event OnComponentBeginOverlap(Sphere)
  (params (OverlappedComponent :type Primitive%20Component%20Object%20Reference) (OtherActor :type Actor%20Object%20Reference) (OtherComp :type Primitive%20Component%20Object%20Reference) (OtherBodyIndex :type Integer) (bFromSweep :type Boolean) (SweepResult :type Hit%20Result%20Structure%20%28by%20ref%29))
  (bind _asmove_to_location (Utilities|Casting|CastToMoveToLocation OtherActor)
    (:then
      (Default|HealthSystem _asmove_to_location 1.0)
      (Audio|PlaySoundatLocation "/Game/Audio/SoundEffects/EnemyDeath.EnemyDeath" "0, 0, 0" "0, 0, 0" 1.0 1.0 0.0 0 0 0)
      (bind _returnvalue (Game|SpawnActorfromClass "/Game/Blueprints/Enemies/DeadEnemy.DeadEnemy_C" (Transformation|GetWorldTransform (Variables|/Game/Blueprints/Enemies/MoveToLocation.MoveToLocation_C|GetMoveToLocation _asmove_to_location)) "Undefined" 0 0))
      (Sprite|SetFlipbook (Variables|/Game/Blueprints/Enemies/DeadEnemy.DeadEnemy_C|GetDeadEnemy _returnvalue) (Variables|/Game/Blueprints/Enemies/MoveToLocation.MoveToLocation_C|GetDeadEnemyFlipbook _asmove_to_location))
      (Actor|DestroyActor _asmove_to_location)
      (bind _assimple_side_scroller_game_instance (Utilities|Casting|CastToSimpleSideScrollerGameInstance (Game|GetGameInstance)))
      (Variables|/Game/Blueprints/Player/SimpleSideScrollerGameInstance.SimpleSideScrollerGameInstance_C|SetScore _assimple_side_scroller_game_instance (+ (Variables|/Game/Blueprints/Player/SimpleSideScrollerGameInstance.SimpleSideScrollerGameInstance_C|GetScore _assimple_side_scroller_game_instance) 100))
      (Actor|DestroyActor))
    (:CastFailed
      (bind _aszig_zag (Utilities|Casting|CastToZigZag OtherActor)
        (:then
          (Default|HealthSystem _aszig_zag 1.0)
          (Audio|PlaySoundatLocation "/Game/Audio/SoundEffects/EnemyDeath.EnemyDeath" "0, 0, 0" "0, 0, 0" 1.0 1.0 0.0 0 0 0)
          (bind _returnvalue_2 (Game|SpawnActorfromClass "/Game/Blueprints/Enemies/DeadEnemy.DeadEnemy_C" (Transformation|GetWorldTransform (Variables|/Game/Blueprints/Enemies/ZigZag.ZigZag_C|GetZigZagEnemy _aszig_zag)) "Undefined" 0 0))
          (Sprite|SetFlipbook (Variables|/Game/Blueprints/Enemies/DeadEnemy.DeadEnemy_C|GetDeadEnemy _returnvalue_2) (Variables|/Game/Blueprints/Enemies/ZigZag.ZigZag_C|GetDeadEnemyFlipbook _aszig_zag))
          (Actor|DestroyActor _aszig_zag)
          (bind _assimple_side_scroller_game_instance_2 (Utilities|Casting|CastToSimpleSideScrollerGameInstance (Game|GetGameInstance)))
          (Variables|/Game/Blueprints/Player/SimpleSideScrollerGameInstance.SimpleSideScrollerGameInstance_C|SetScore _assimple_side_scroller_game_instance_2 (+ (Variables|/Game/Blueprints/Player/SimpleSideScrollerGameInstance.SimpleSideScrollerGameInstance_C|GetScore _assimple_side_scroller_game_instance_2) 250))
          (Actor|DestroyActor))
        (:CastFailed
          (bind _asmove_to_player (Utilities|Casting|CastToMoveToPlayer OtherActor)
            (:then
              (Default|HealthSystem _asmove_to_player 1.0)
              (Audio|PlaySoundatLocation "/Game/Audio/SoundEffects/EnemyDeath.EnemyDeath" "0, 0, 0" "0, 0, 0" 1.0 1.0 0.0 0 0 0)
              (bind _returnvalue_3 (Game|SpawnActorfromClass "/Game/Blueprints/Enemies/DeadEnemy.DeadEnemy_C" (Transformation|GetWorldTransform (Variables|/Game/Blueprints/Enemies/MoveToPlayer.MoveToPlayer_C|GetMoveToPlayerEnemy _asmove_to_player)) "Undefined" 0 0))
              (Sprite|SetFlipbook (Variables|/Game/Blueprints/Enemies/DeadEnemy.DeadEnemy_C|GetDeadEnemy _returnvalue_3) (Variables|/Game/Blueprints/Enemies/MoveToPlayer.MoveToPlayer_C|GetDeadEnemyFlipbook _asmove_to_player))
              (Actor|DestroyActor _asmove_to_player)
              (bind _assimple_side_scroller_game_instance_3 (Utilities|Casting|CastToSimpleSideScrollerGameInstance (Game|GetGameInstance)))
              (Variables|/Game/Blueprints/Player/SimpleSideScrollerGameInstance.SimpleSideScrollerGameInstance_C|SetScore _assimple_side_scroller_game_instance_3 (+ (Variables|/Game/Blueprints/Player/SimpleSideScrollerGameInstance.SimpleSideScrollerGameInstance_C|GetScore _assimple_side_scroller_game_instance_3) 1000))
              (Actor|DestroyActor))
            (:CastFailed
              (bind _asrotating (Utilities|Casting|CastToRotating OtherActor)
                (:then
                  (Default|HealthSystem _asrotating 1.0)
                  (Audio|PlaySoundatLocation "/Game/Audio/SoundEffects/EnemyDeath.EnemyDeath" "0, 0, 0" "0, 0, 0" 1.0 1.0 0.0 0 0 0)
                  (bind _returnvalue_4 (Game|SpawnActorfromClass "/Game/Blueprints/Enemies/DeadEnemy.DeadEnemy_C" (Transformation|GetWorldTransform (Variables|/Game/Blueprints/Enemies/Rotating.Rotating_C|GetRotatingEnemy _asrotating)) "Undefined" 0 0))
                  (Sprite|SetFlipbook (Variables|/Game/Blueprints/Enemies/DeadEnemy.DeadEnemy_C|GetDeadEnemy _returnvalue_4) (Variables|/Game/Blueprints/Enemies/Rotating.Rotating_C|GetDeadEnemyFlipbook _asrotating))
                  (Actor|DestroyActor _asrotating)
                  (bind _assimple_side_scroller_game_instance_4 (Utilities|Casting|CastToSimpleSideScrollerGameInstance (Game|GetGameInstance)))
                  (Variables|/Game/Blueprints/Player/SimpleSideScrollerGameInstance.SimpleSideScrollerGameInstance_C|SetScore _assimple_side_scroller_game_instance_4 (+ (Variables|/Game/Blueprints/Player/SimpleSideScrollerGameInstance.SimpleSideScrollerGameInstance_C|GetScore _assimple_side_scroller_game_instance_4) 500))
                  (Actor|DestroyActor))
                (:CastFailed
                  (bind _asboss (Utilities|Casting|CastToBoss OtherActor))
                  (Default|HealthSystem _asboss 1.0)
                  (Audio|PlaySoundatLocation "/Game/Audio/SoundEffects/EnemyDeath.EnemyDeath" "0, 0, 0" "0, 0, 0" 1.0 1.0 0.0 0 0 0)
                  (bind _returnvalue_5 (Game|SpawnActorfromClass "/Game/Blueprints/Enemies/DeadEnemy.DeadEnemy_C" (Transformation|GetWorldTransform (Variables|/Game/Blueprints/Enemies/Boss.Boss_C|GetBossEnemy _asboss)) "Undefined" 0 0))
                  (Sprite|SetFlipbook (Variables|/Game/Blueprints/Enemies/DeadEnemy.DeadEnemy_C|GetDeadEnemy _returnvalue_5) (Variables|/Game/Blueprints/Enemies/Boss.Boss_C|GetDeadEnemyFlipbook _asboss))
                  (Actor|DestroyActor _asboss)
                  (bind _assimple_side_scroller_game_instance_5 (Utilities|Casting|CastToSimpleSideScrollerGameInstance (Game|GetGameInstance)))
                  (Variables|/Game/Blueprints/Player/SimpleSideScrollerGameInstance.SimpleSideScrollerGameInstance_C|SetScore _assimple_side_scroller_game_instance_5 (+ (Variables|/Game/Blueprints/Player/SimpleSideScrollerGameInstance.SimpleSideScrollerGameInstance_C|GetScore _assimple_side_scroller_game_instance_5) 10000))
                  (Game|SpawnActorfromClass "/Game/Blueprints/Items/PickupKeys.PickupKeys_C" (Math|Conversions|ToTransform(Vector) (Transformation|GetActorLocation)) "Undefined" 0 0)
                  (Actor|DestroyActor))))))))))

(fn ConstructionScript
  (Actor|SetLifeSpan 5.0))
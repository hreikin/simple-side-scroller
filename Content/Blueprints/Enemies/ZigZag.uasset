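; ZigZag enemy for a side-scroller that hurts the player on contact and moves via an InterpToMovement component.
; While it is alive, overlap launches the character upward and calls its HealthSystem for one damage.
; Its own HealthSystem subtracts damage and marks it dead only when health equals exactly zero.
; UnfreezeEnemy re-enables movement ticking after a delay, the construction script tints the sprite, and UpdateAnimation is empty.
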(event OnComponentBeginOverlap(ZigZagEnemy)
  (params (OverlappedComponent :type Primitive%20Component%20Object%20Reference) (OtherActor :type Actor%20Object%20Reference) (OtherComp :type Primitive%20Component%20Object%20Reference) (OtherBodyIndex :type Integer) (bFromSweep :type Boolean) (SweepResult :type Hit%20Result%20Structure%20%28by%20ref%29))
  (if (not (Variables|EnemyControls|GetIsDead))
    (bind _assimple_side_scroller_character (Utilities|Casting|CastToSimpleSideScrollerCharacter OtherActor))
    (Character|LaunchCharacter _assimple_side_scroller_character "0.000000,0.000000,500.000000" true true)
    (Default|HealthSystem _assimple_side_scroller_character 1.0)))

(event Custom|HealthSystem
  (params (Damage :type Float%20%28single-precision%29))
  (bind _output_get (Variables|EnemyControls|SetEnemyHealth (- (Variables|EnemyControls|GetEnemyHealth) Damage)))
  (if (== _output_get 0.0)
    (Variables|EnemyControls|SetIsDead true)))

(event Custom|UnfreezeEnemy
  (Utilities|FlowControl|Delay 1e+01)
  (Components|Tick|SetComponentTickEnabled (Variables|Default|GetInterpToMovement) true))

(fn ConstructionScript
  (Sprite|SetSpriteColor (Variables|Default|GetZigZagEnemy) (Variables|EnemyControls|GetEnemyColour)))

(fn UpdateAnimation)
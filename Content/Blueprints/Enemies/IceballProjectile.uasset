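; Iceball projectile that freezes the enemy it overlaps, then destroys itself.
; The sphere overlap runs a cast chain over five types: MoveToPlayer and Boss get a frozen flag, while MoveToLocation, Rotating and ZigZag have their movement halted directly.
; MoveToLocation and ZigZag also receive an UnfreezeEnemy call right after the halt.
; Other actors are ignored, and the construction script sets a short lifespan to remove stray shots.
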(event OnComponentBeginOverlap(Sphere)
  (params (OverlappedComponent :type Primitive%20Component%20Object%20Reference) (OtherActor :type Actor%20Object%20Reference) (OtherComp :type Primitive%20Component%20Object%20Reference) (OtherBodyIndex :type Integer) (bFromSweep :type Boolean) (SweepResult :type Hit%20Result%20Structure%20%28by%20ref%29))
  (bind _asmove_to_player (Utilities|Casting|CastToMoveToPlayer OtherActor)
    (:then
      (Variables|/Game/Blueprints/Enemies/MoveToPlayer.MoveToPlayer_C|SetEnemyFrozen _asmove_to_player true))
    (:CastFailed
      (bind _asboss (Utilities|Casting|CastToBoss OtherActor)
        (:then
          (Variables|/Game/Blueprints/Enemies/Boss.Boss_C|SetEnemyFrozen _asboss true))
        (:CastFailed
          (bind _asmove_to_location (Utilities|Casting|CastToMoveToLocation OtherActor)
            (:then
              (Audio|Components|Audio|Stop (Variables|/Game/Blueprints/Enemies/MoveToLocation.MoveToLocation_C|GetLiftTimeLine _asmove_to_location))
              (Default|UnfreezeEnemy _asmove_to_location))
            (:CastFailed
              (bind _asrotating (Utilities|Casting|CastToRotating OtherActor)
                (:then
                  (Components|Activation|Deactivate (Variables|/Game/Blueprints/Enemies/Rotating.Rotating_C|GetRotatingMovement _asrotating)))
                (:CastFailed
                  (bind _aszig_zag (Utilities|Casting|CastToZigZag OtherActor))
                  (Components|Tick|SetComponentTickEnabled (Variables|/Game/Blueprints/Enemies/ZigZag.ZigZag_C|GetInterpToMovement _aszig_zag) false)
                  (Default|UnfreezeEnemy _aszig_zag)))))))))
  (Actor|DestroyActor))

(fn ConstructionScript
  (Actor|SetLifeSpan 5.0))
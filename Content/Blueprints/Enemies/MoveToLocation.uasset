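; Side-scroller enemy whose sprite patrols between its origin and EndLocation and, while alive, launches and damages the player on overlap.
; A timeline paced by TravelTimeSeconds lerps the sprite, with LiftForward and LiftBackwards flipping its rotation and alternating after StopDelay.
; UnfreezeEnemy resumes the timeline after a delay, and HealthSystem marks the enemy dead at zero health.
; The construction script applies EnemyColour and can preview the end position via TestEndLocation.
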(event OnComponentBeginOverlap(MoveToLocation)
  (params (OverlappedComponent :type Primitive%20Component%20Object%20Reference) (OtherActor :type Actor%20Object%20Reference) (OtherComp :type Primitive%20Component%20Object%20Reference) (OtherBodyIndex :type Integer) (bFromSweep :type Boolean) (SweepResult :type Hit%20Result%20Structure%20%28by%20ref%29))
  (if (not (Variables|EnemyControls|GetIsDead))
    (bind _assimple_side_scroller_character (Utilities|Casting|CastToSimpleSideScrollerCharacter OtherActor))
    (Character|LaunchCharacter _assimple_side_scroller_character "0.000000,0.000000,500.000000" true true)
    (Default|HealthSystem _assimple_side_scroller_character 1.0)))

(event Custom|HealthSystem
  (params (Damage :type Float%20%28single-precision%29))
  (bind _output_get (Variables|EnemyControls|SetEnemyHealth (- (Variables|EnemyControls|GetEnemyHealth) Damage)))
  (if (== _output_get 0.0)
    (Variables|EnemyControls|SetIsDead true)))

(event Custom|LiftBackwards
  (Transformation|SetRelativeRotation (Variables|Default|GetMoveToLocation) "0, 0, 0" false false)
  (bind (_direction _driver) (Timeline|LiftTimeLine ReverseFromEnd)
    (:Update
      (Transformation|SetRelativeLocation (Variables|Default|GetMoveToLocation) (Math|Vector|Lerp(Vector) "0, 0, 0" (Variables|EnemyControls|GetEndLocation) _driver) false false))
    (:Finished
      (Utilities|FlowControl|Delay (Variables|EnemyControls|GetStopDelay))
      (switch Utilities|FlowControl|Switch|SwitchonETimelineDirection _direction
        (:Forward
          (CallFunction|LiftBackwards))
        (:Backward
          (CallFunction|LiftForward))))))

(event Custom|LiftForward
  (Transformation|SetRelativeRotation (Variables|Default|GetMoveToLocation) "0,180.000000, 0" false false)
  (bind (_direction _driver) (Timeline|LiftTimeLine PlayFromStart)
    (:Update
      (Transformation|SetRelativeLocation (Variables|Default|GetMoveToLocation) (Math|Vector|Lerp(Vector) "0, 0, 0" (Variables|EnemyControls|GetEndLocation) _driver) false false))
    (:Finished
      (Utilities|FlowControl|Delay (Variables|EnemyControls|GetStopDelay))
      (switch Utilities|FlowControl|Switch|SwitchonETimelineDirection _direction
        (:Forward
          (CallFunction|LiftBackwards))
        (:Backward
          (CallFunction|LiftForward))))))

(event Custom|UnfreezeEnemy
  (Utilities|FlowControl|Delay 1e+01)
  (bind (_direction _driver) (Timeline|LiftTimeLine Play)
    (:Update
      (Transformation|SetRelativeLocation (Variables|Default|GetMoveToLocation) (Math|Vector|Lerp(Vector) "0, 0, 0" (Variables|EnemyControls|GetEndLocation) _driver) false false))
    (:Finished
      (Utilities|FlowControl|Delay (Variables|EnemyControls|GetStopDelay))
      (switch Utilities|FlowControl|Switch|SwitchonETimelineDirection _direction
        (:Forward
          (CallFunction|LiftBackwards))
        (:Backward
          (CallFunction|LiftForward))))))

(event EventBeginPlay
  (bind _lifttimeline (Variables|Default|GetLiftTimeLine))
  (Components|Timeline|SetPlayRate (Variables|Default|GetLiftTimeLine) (/ 1.0 (Variables|EnemyControls|GetTravelTimeSeconds)))
  (Variables|EnemyControls|SetTestEndLocation true)
  (if (Audio|Components|Audio|IsPlaying _lifttimeline)
    (if (Class|TimelineComponent|IsReversing _lifttimeline)
      (bind (_direction _driver) (Timeline|LiftTimeLine Play)
        (:Update
          (Transformation|SetRelativeLocation (Variables|Default|GetMoveToLocation) (Math|Vector|Lerp(Vector) "0, 0, 0" (Variables|EnemyControls|GetEndLocation) _driver) false false))
        (:Finished
          (Utilities|FlowControl|Delay (Variables|EnemyControls|GetStopDelay))
          (switch Utilities|FlowControl|Switch|SwitchonETimelineDirection _direction
            (:Forward
              (CallFunction|LiftBackwards))
            (:Backward
              (CallFunction|LiftForward)))))
      (else
        (Timeline|LiftTimeLine Reverse)))))

(fn ConstructionScript
  (Transformation|SetRelativeLocation (Variables|Default|GetMoveToLocation) (Math|Vector|SelectVector (Variables|EnemyControls|GetEndLocation) "0, 0, 0" (Variables|EnemyControls|GetTestEndLocation)) false false)
  (Sprite|SetSpriteColor (Variables|Default|GetMoveToLocation) (Variables|EnemyControls|GetEnemyColour)))

(fn UpdateAnimation)